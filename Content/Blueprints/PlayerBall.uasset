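; Player-controlled physics ball that is launched along the camera's aim by a hold-and-release charged impulse, only while grounded.
; Tick makes the actor trail the simulated sphere, sets damping from the traced ground surface, and blends to first person when the ball rests on flat ground.
; Hard hits play bounce sounds, and flat landings zero velocity.
; Ball state and timer save every frame and restore on BeginPlay; pausing displays the timer.
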(event `self.ReceiveBeginPlay`
  (bind _sphere (`self.Sphere`))
  ;[1 1 1] Load Save Game
  (bind _returnvalue (`GameplayStatics.LoadGameFromSlot` "Main"))
  (bind _asmain_save_game (cast `/Game/Blueprints/MainSaveGame` _returnvalue))
  (`SceneComponent.K2_SetWorldLocation` _sphere (`/Game/Blueprints/MainSaveGame.BallPosition` _asmain_save_game) false true)
  (`PrimitiveComponent.SetAllPhysicsAngularVelocityInRadians` _sphere (`/Game/Blueprints/MainSaveGame.BallRotVelocity` _asmain_save_game) false)
  (`PrimitiveComponent.SetAllPhysicsLinearVelocity` _sphere (`/Game/Blueprints/MainSaveGame.BallLinVelocity` _asmain_save_game) false)
  (set `self.Time` (`/Game/Blueprints/MainSaveGame.STime` _asmain_save_game)))

(event `InputAction|Pause Game` :paused true
  (params (Key :type "Key Structure"))
  (bind _returnvalue (`GameplayStatics.GetPlayerController` 0))
  (bind _returnvalue_2 (`GameplayStatics.GetPlayerController` 0))
  (bind _pause_menu_reference (`self.Pause Menu Reference`))
  ;[1 1 1] Pause
  (:`Pressed`
    (`/Engine/EditorBlueprintResources/StandardMacros.IsValid` (`self.Pause Menu Reference`)
      (:`Is Valid`
        _)
      (:`Is Not Valid`
        (bind _returnvalue_3 (`|CreateWidget` "/Game/Blueprints/UI/PauseMenu.PauseMenu_C"))
        (set `self.Pause Menu Reference` _returnvalue_3)))
    (if (`GameplayStatics.IsGamePaused`)
      (`Widget.RemoveFromParent` _pause_menu_reference)
      (`GameplayStatics.SetGamePaused` false)
      (set `PlayerController.bShowMouseCursor` false _returnvalue)
      (`WidgetBlueprintLibrary.SetInputMode_GameOnly` _returnvalue)
      (else
        (set `/Game/Blueprints/UI/PauseMenu.DisplayTime` (`self.Time`) _pause_menu_reference)
        (`UserWidget.AddToViewport` _pause_menu_reference 0)
        (`GameplayStatics.SetGamePaused` true)
        (set `PlayerController.bShowMouseCursor` true _returnvalue_2)
        (`WidgetBlueprintLibrary.SetInputMode_GameAndUIEx` _returnvalue_2 _pause_menu_reference "LockInFullscreen" false)))))

(event `self.ReceiveHit`
  (params (MyComp :type "PrimitiveComponent Object Reference") (Other :type "Actor Object Reference") (OtherComp :type "PrimitiveComponent Object Reference") (bSelfMoved :type Boolean) (HitLocation :type "Vector Structure") (HitNormal :type "Vector Structure") (NormalImpulse :type "Vector Structure") (Hit :type "HitResult Structure (by ref)"))
  (bind _sphere (`self.Sphere`))
  ;[1 1 1] Play Bouncing Sound
  (if (not (< (`KismetMathLibrary.VSize` NormalImpulse) 2000.0))
    (`GameplayStatics.PlaySoundAtLocation` "/Game/Sounds/BallKick1.BallKick1" HitLocation (struct) (/ (/ (`KismetMathLibrary.VSize` (`SceneComponent.GetComponentVelocity` MyComp)) (`self.ShootingSpeed`)) (`self.MaxShootingChargeTime`)) 1.0 0.0 null null null null)
    ;[1 1 1] Stop Ball on Landing
    (if (> (.z HitNormal) 0.999)
      (`PrimitiveComponent.SetAllPhysicsLinearVelocity` _sphere (0.0 0.0 0.0) false)
      (`PrimitiveComponent.SetAllPhysicsAngularVelocityInDegrees` _sphere (`KismetMathLibrary.MakeVector` 0.0) false))))

(event `self.ReceiveTick`
  (params (DeltaSeconds :type "Float (single-precision)"))
  (bind _sphere (`self.Sphere`))
  (bind _relativelocation (`SceneComponent.RelativeLocation` (`self.Sphere`)))
  (bind _relativelocation_2 (`SceneComponent.RelativeLocation` (`self.Sphere`)))
  (bind _returnvalue (`KismetMathLibrary.VSize` (`SceneComponent.GetComponentVelocity` (`self.Sphere`))))
  ;[1 1 1] Saving the current state
  (bind _returnvalue_2 (`GameplayStatics.CreateSaveGameObject` "/Game/Blueprints/MainSaveGame.MainSaveGame_C"))
  (set `/Game/Blueprints/MainSaveGame.BallPosition` (`SceneComponent.K2_GetComponentLocation` _sphere) _returnvalue_2)
  (bind _returnvalue_3 (`PrimitiveComponent.GetPhysicsLinearVelocity` _sphere "None"))
  (set `/Game/Blueprints/MainSaveGame.BallRotVelocity` (`PrimitiveComponent.GetPhysicsAngularVelocityInRadians` _sphere "None") _returnvalue_2)
  (set `/Game/Blueprints/MainSaveGame.BallLinVelocity` _returnvalue_3 _returnvalue_2)
  (set `/Game/Blueprints/MainSaveGame.STime` (`self.Time`) _returnvalue_2)
  (`GameplayStatics.SaveGameToSlot` _returnvalue_2 "Main")
  (set `self.Time` (+ (`self.Time`) DeltaSeconds))
  ;[1 1 1] Keep ball and actor linked
  (`self.K2_SetActorLocation` (`KismetMathLibrary.VInterpTo` (`self.K2_GetActorLocation` self) (`SceneComponent.K2_GetComponentLocation` (`self.Sphere`)) DeltaSeconds 20.0))
  ;[1 1 1] Switch Camera from 3rd person to 1st person when Ball is standing still
  (bind _outhit (`KismetSystemLibrary.LineTraceSingle` _relativelocation (+ _relativelocation (* (`KismetMathLibrary.Vector_Down`) (25.0 25.0 25.0))) "TraceTypeQuery1" false (`|MakeArray` self :!type "Actor Object Reference")))
  (if (or (< (.z (`.Normal` (`GameplayStatics.BreakHitResult` _outhit))) 0.99999) (or (or (> (`self.SpeedLastFrame`) 7.0) (> _returnvalue 7.0)) (not (`self.IsTouchingGround`))))
    (`self.TransitionToThirdPerson` DeltaSeconds)
    (else
      (`self.TransitionToFirstPerson` DeltaSeconds)))
  (set `self.SpeedLastFrame` _returnvalue)
  ;[1 1 1] Check if touching ground
  (bind _outhits (`KismetSystemLibrary.SphereTraceMulti` _relativelocation_2 (+ _relativelocation_2 (* (`KismetMathLibrary.Vector_Down`) (8.0 8.0 8.0))) 15.0 "TraceTypeQuery1" false (`|MakeArray` self :!type "Actor Object Reference")))
  (set `self.IsTouchingGround` (> (`KismetArrayLibrary.Array_Length` _outhits) 0))
  (`self.Set Damping` (`GameplayStatics.GetSurfaceType` (`|GetArrayItem` _outhits))))

(event `InputAxis|Turn` :overrideparent false
  (params (AxisValue :type "Float (single-precision)"))
  ;[1 1 1] Camera Controls
  (`self.AddControllerYawInput` AxisValue))

(event `InputAction|Shoot`
  (params (Key :type "Key Structure"))
  (bind _returnvalue (`KismetSystemLibrary.GetGameTimeInSeconds`))
  (bind _returnvalue_2 (`KismetMathLibrary.FMin` (/ (`self.TimeLMBHeld`) (`self.MaxShootingChargeTime`)) 1.0))
  ;[1 1 1] Shooting The Ball
  (:`Pressed`
    (set `self.TimeWhenPressed` _returnvalue))
  (:`Released`
    (if (`self.IsTouchingGround`)
      (set `self.TimeLMBHeld` (- _returnvalue (`self.TimeWhenPressed`)))
      (`PrimitiveComponent.AddImpulse` (`self.Sphere`) (* (`SceneComponent.GetForwardVector` (`self.Camera`)) (* _returnvalue_2 (`self.ShootingSpeed`))) "None" true)
      (`GameplayStatics.PlaySoundAtLocation` "/Game/Sounds/BallKick1.BallKick1" (`self.K2_GetActorLocation`) (struct) _returnvalue_2 1.0 0.0 null null null null))))

(event `InputAxis|LookUp` :overrideparent false
  (params (AxisValue :type "Float (single-precision)"))
  ;[1 1 1] Camera Controls
  (`self.AddControllerPitchInput` AxisValue))

(fn `Set Damping`
  (params (GroundActor :type "EPhysicalSurface Enum" :default "SurfaceType_Default"))
  (bind _sphere (`self.Sphere`))
  (switch `EPhysicalSurface` GroundActor
    (:`SurfaceType_Default`
      (`PrimitiveComponent.SetAngularDamping` _sphere 2.0)
      (`PrimitiveComponent.SetLinearDamping` _sphere 0.1))
    (:`SurfaceType1`
      (`PrimitiveComponent.SetAngularDamping` _sphere 10.0)
      (`PrimitiveComponent.SetLinearDamping` _sphere 3.0))
    (:`SurfaceType2`
      (`PrimitiveComponent.SetAngularDamping` _sphere 3.0)
      (`PrimitiveComponent.SetLinearDamping` _sphere 0.3))
    (:`SurfaceType3`
      (`PrimitiveComponent.SetAngularDamping` _sphere 50.0)
      (`PrimitiveComponent.SetLinearDamping` _sphere 5.0))
    (:`SurfaceType4`
      (`PrimitiveComponent.SetAngularDamping` _sphere 1.5)
      (`PrimitiveComponent.SetLinearDamping` _sphere 0.05))
    (:`SurfaceType6`
      (`PrimitiveComponent.SetAngularDamping` _sphere 9999999.0)
      (`PrimitiveComponent.SetLinearDamping` _sphere 0.0))))

(fn `TransitionToFirstPerson`
  (params (DeltaTime :type "Float (double-precision)"))
  (bind _cameraspring (`self.CameraSpring`))
  (`SceneComponent.SetVisibility` (`self.Sphere`) false false)
  (set `SpringArmComponent.TargetArmLength` (`KismetMathLibrary.FInterpTo` (`SpringArmComponent.TargetArmLength` _cameraspring) 0.0 DeltaTime 30.0) _cameraspring)
  (set `SpringArmComponent.SocketOffset` (`KismetMathLibrary.VInterpTo` (`SpringArmComponent.SocketOffset` _cameraspring) (0.0 0.0 0.0) DeltaTime 30.0) _cameraspring))

(fn `TransitionToThirdPerson`
  (params (DeltaTime :type "Float (double-precision)"))
  (bind _cameraspring (`self.CameraSpring`))
  (`SceneComponent.SetVisibility` (`self.Sphere`) true false)
  (set `SpringArmComponent.TargetArmLength` (`KismetMathLibrary.FInterpTo` (`SpringArmComponent.TargetArmLength` _cameraspring) 300.0 DeltaTime 30.0) _cameraspring)
  (set `SpringArmComponent.SocketOffset` (`KismetMathLibrary.VInterpTo` (`SpringArmComponent.SocketOffset` _cameraspring) (0.0 0.0 70.0) DeltaTime 30.0) _cameraspring))

(fn `UserConstructionScript`)